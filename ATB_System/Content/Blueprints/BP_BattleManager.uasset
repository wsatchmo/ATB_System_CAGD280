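; Battle manager that runs turn-based combat between the level's heroes and enemies.
; On BeginPlay it switches view to the battle camera, gathers both parties, creates a UI-focused HUD, then adds each hero to it and starts their turn timer.
; TurnCreator queues characters uniquely in TurnOrder.
; A DoOnce gate runs one turn at a time, binding to each character's TurnOver dispatcher, and NextTurn resets it.
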(event `self.ReceiveBeginPlay`
  (`self.SetBattleCamera`)
  (`self.CreateParties`)
  (`self.AddBattleWidget`)
  (`self.AddPartyToHUD`))

(event `SetBattleCamera`
  ;[0 0 0.6431 0.502] Set the Battle Cam to look at the Player Controller
  (bind _returnvalue (`GameplayStatics.GetActorOfClass` "/Game/Blueprints/BattleObjects/BP_BattleCamera.BP_BattleCamera_C"))
  (bind _output_get (set `self.BattleCam` _returnvalue))
  (`PlayerController.SetViewTargetWithBlend` (`GameplayStatics.GetPlayerController` 0) _output_get 0.0 "VTBlend_Linear" 0.0 false))

(event `CreateParties`
  ;[0.09412 0.6431 0.1255 0.502] Create parties based on Base Heroes and Base Enemies
  (bind _outactors (`GameplayStatics.GetAllActorsOfClass` "/Game/Blueprints/Characters/Heroes/BP_BaseHero.BP_BaseHero_C"))
  (set `self.PlayerParty` _outactors)
  (bind _outactors_2 (`GameplayStatics.GetAllActorsOfClass` "/Game/Blueprints/Characters/Enemies/BP_BaseEnemy.BP_BaseEnemy_C"))
  (set `self.EnemyParty` _outactors_2))

(event `AddBattleWidget`
  ;[0 0 0.6431 0.502] Add the HUD widget to the screen
  (bind _returnvalue (`|CreateWidget` "/Game/Blueprints/UI_Elements/WBP_HUD.WBP_HUD_C" (`GameplayStatics.GetPlayerController` 0)))
  (bind _output_get (set `self.HUD` _returnvalue))
  (`UserWidget.AddToViewport` _output_get 0)
  (`WidgetBlueprintLibrary.SetInputMode_UIOnlyEx` (`GameplayStatics.GetPlayerController` 0) (`self.HUD`)))

(event `AddPartyToHUD`
  ;[0.09412 0.6431 0.1255 0.502] Dynamically adds each character in the party to the HUD using the function in WBP HUD & starts its Turn Timer function
  (for _array_element (`self.PlayerParty`)
    (`/Game/Blueprints/UI_Elements/WBP_HUD.AddCharacterToHUD` (`self.HUD`) _array_element)
    (`/Game/Blueprints/Characters/BP_BaseCharacter.TurnTimer` _array_element)))

(event `TurnCreator`
  (params (Character :type "/Game/Blueprints/Characters/BP_BaseCharacter Object Reference"))
  ; Creates turn order from Characters' speed
  (`KismetArrayLibrary.Array_AddUnique` (`self.TurnOrder`) Character)
  (`self.ThisTurn`))

(event `ThisTurn`
  (bind _turnorder (`self.TurnOrder`))
  (bind _output (`|GetArrayItem` _turnorder))
  ; Handles one turn by checking if charcter on index is valid, calling its StartTurn function, binding to TurnOver dispatcher and removing it from the array index 0
  (`/Engine/EditorBlueprintResources/StandardMacros.DoOnce` false :!label _label
    (:`Completed`
      (if (`KismetArrayLibrary.Array_IsValidIndex` _turnorder)
        (`/Game/Blueprints/Characters/BP_BaseCharacter.StartTurn` _output)
        (add `/Game/Blueprints/Characters/BP_BaseCharacter.TurnOver` _output (`|CreateDelegate` :!event `NextTurn`))
        (`KismetArrayLibrary.Array_Remove` (`self.TurnOrder`))
        (else
          (`self.NextTurn`))))))

(event `NextTurn`
  ; Starting the next turn...
  (`|ExecutionSequence`
    (:`then_0`
      (goto _label :!via `Reset`))
    (:`then_1`
      ; ...by resetting the process with the new character at index 0
      (if (`KismetArrayLibrary.Array_IsValidIndex` (`self.TurnOrder`))
        (`self.ThisTurn`)))))

(fn `UserConstructionScript`)