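; Base character for a turn-based battle system with speed-driven action timers, shared by heroes and enemies.
; Non-enemies get Enhanced Input movement; construction tints the cube and finds the BattleManager.
; StartTurn gives heroes a battle menu and orbiting camera; attacks stop the orbit, with melee ending the turn after a delay and ranged still empty.
; EndTurn signals turn over and starts a Speed-based, minimum-clamped timer that requests the next turn from the BattleManager.
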(event `self.ReceiveBeginPlay`
  ;[0 0 0 0.5] MOVEMENT
  ;;[0.08236 0.3781 0.1393 0.5] Set ref to self, player controller & add mapping context (only if this is NOT an enemy)
  (set `self.Character` self)
  (if (not (`self.IsEnemy`))
    (bind _asbp_player_controller (cast `/Game/Blueprints/BP_PlayerController` (`GameplayStatics.GetPlayerController` 0)))
    (bind _output_get (set `self.PlayerController` _asbp_player_controller))
    (bind _returnvalue (pcsubsystem `EnhancedInputLocalPlayerSubsystem` _output_get))
    (`/Engine/EditorBlueprintResources/StandardMacros.IsValid` _returnvalue
      (:`Is Valid`
        (`EnhancedInputSubsystemInterface.AddMappingContext` _returnvalue "/Game/Inputs/IMC_PlayerControls.IMC_PlayerControls" 0 (struct))))))

(event `EnhancedInput|/Game/Inputs/Actions/IA_Move`
  (params (ActionValue :type "Vector2D Structure") (ElapsedSeconds :type "Float (double-precision)") (TriggeredSeconds :type "Float (double-precision)") (InputAction :type "InputAction Object Reference" :default "/Game/Inputs/Actions/IA_Move.IA_Move"))
  (bind (_returnvalue_roll _returnvalue_pitch _returnvalue_yaw) (`KismetMathLibrary.BreakRotator` (`self.GetControlRotation`)))
  (bind (_returnvalue_roll_2 _returnvalue_pitch_2 _returnvalue_yaw_2) (`KismetMathLibrary.BreakRotator` (`self.GetControlRotation`)))
  ;[0 0 0 0.5] MOVEMENT
  ;;[0.08236 0.3781 0.1393 0.5] Move with enhanced input
  (:`Triggered`
    (`self.AddMovementInput` (`KismetMathLibrary.GetRightVector` (`KismetMathLibrary.MakeRotator` _returnvalue_roll_2 0.0 _returnvalue_yaw_2)) ActionValue_X)
    (`self.AddMovementInput` (`KismetMathLibrary.GetForwardVector` (`KismetMathLibrary.MakeRotator` _returnvalue_roll 0.0 _returnvalue_yaw)) ActionValue_Y)))

(event `AttackCommand`
  ;[0 0 0 0.5] COMBAT
  ;;[0.5961 0 0 0.502] Select who to look at, turn off orbit, and check for ranged or melee attack
  (message `/Game/Blueprints/BattleObjects/BPI_DynamicCameraInterface.SetOrbit` (`Controller.GetViewTarget` (`GameplayStatics.GetPlayerController` 0)) false)
  (if (`self.IsRanged`)
    (`self.RangedAttack`)
    (else
      (`self.MeleeAttack`))))

(event `MeleeAttack`
  ;[0 0 0 0.5] COMBAT
  ;;[0.5961 0 0 0.502] INITIANE MELEE ATTACK
  ;;; Remove menu so it can't be clicked again
  ;;;; ActionsMenu instead?
  (bind _battlemenu (`self.BattleMenu`)
    (:`then`
      (`Widget.RemoveFromParent` _battlemenu)
      (`KismetSystemLibrary.Delay` 1.6)
      (`self.EndTurn`))
    (:`else`)))

(event `RangedAttack`
  ;[0 0 0 0.5] COMBAT
  ;;[0.5961 0 0 0.502] INITATE RANGED ATTACK
)

(fn `EndTurn`
  (`self.TurnOver`)
  (`self.TurnTimer`))

(fn `RequestTurn`
  ; Creates this character's turn in the Battlemanager
  (`/Game/Blueprints/BP_BattleManager.TurnCreator` (`self.BattleManager`) (`self.Character`)))

(fn `SetCamera`
  (bind _returnvalue (`GameplayStatics.GetActorOfClass` "/Game/Blueprints/BattleObjects/BP_DynamicCamera.BP_DynamicCamera_C"))
  (`PlayerController.SetViewTargetWithBlend` (`GameplayStatics.GetPlayerController` 0) _returnvalue 0.0 "VTBlend_Linear" 0.0 false)
  (message `/Game/Blueprints/BattleObjects/BPI_DynamicCameraInterface.SetDynamicLocation` _returnvalue (`self.Character`) (0.0 0.0 0.0))
  (message `/Game/Blueprints/BattleObjects/BPI_DynamicCameraInterface.SetOrbit` (`Controller.GetViewTarget` (`GameplayStatics.GetPlayerController` 0)) true))

(fn `StartTurn`
  ; Add Battle menus to screen
  (if (`KismetMathLibrary.ClassIsChildOf` (`GameplayStatics.GetObjectClass` (`self.Character`)) "/Game/Blueprints/Characters/Heroes/BP_BaseHero.BP_BaseHero_C")
    (bind _returnvalue (`|CreateWidget` "/Game/Blueprints/UI_Elements/WBP_BattleMenu.WBP_BattleMenu_C" null (`self.Character`)))
    (bind _output_get (set `self.BattleMenu` _returnvalue))
    (`UserWidget.AddToViewport` _output_get 0)
    (`self.SetCamera`)))

(fn `TurnTimer`
  (bind _minactiontime (`self.MinActionTime`))
  ; Set timer based on Speed & set ActionTimer for progress bar
  (if (<= (- (`self.MaxActionTime`) (`self.Speed`)) _minactiontime)
    (bind _returnvalue (`KismetSystemLibrary.K2_SetTimer` self "RequestTurn" _minactiontime))
    (set `self.ActionTimer` _returnvalue)
    (else
      (bind _returnvalue_2 (`KismetSystemLibrary.K2_SetTimer` self "RequestTurn" (- (`self.MaxActionTime`) (`self.Speed`))))
      (set `self.ActionTimer` _returnvalue_2))))

(fn `UserConstructionScript`
  (`|ExecutionSequence`
    (:`then_0`
      ; Create dynamic Hero color parameter
      (bind _returnvalue (`PrimitiveComponent.CreateDynamicMaterialInstance` (`self.Cube`) 0 "/Game/Materials/M_Hero.M_Hero" "None"))
      (`MaterialInstanceDynamic.SetVectorParameterValue` _returnvalue "Color" (`self.Color`)))
    (:`then_1`
      ; Get and set a ref to BattleManager
      (bind _asbp_battle_manager (castclass `/Game/Blueprints/BP_BattleManager` "/Game/Blueprints/BP_BattleManager.BP_BattleManager_C"))
      (bind _returnvalue_2 (`GameplayStatics.GetActorOfClass` _asbp_battle_manager))
      (set `self.BattleManager` _returnvalue_2))))