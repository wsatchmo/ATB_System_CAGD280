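; BP_DynamicCamera is a battle camera actor on a spring arm that can follow an actor, glide to a location or orbit.
; SetDynamicLocation snaps and attaches it to a valid actor, zeroing the camera's relative rotation, or otherwise stores a target location.
; While unattached, Tick eases toward that location with VInterpTo.
; SetOrbit toggles slow yaw spin through RotatingMovement and spring arm yaw inheritance, resetting actor rotation when off.
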(event `/Game/Blueprints/BattleObjects/BPI_DynamicCameraInterface.SetOrbit`
  (params (IsOrbiting :type Boolean))
  ; USING UNTERFACE : If IsOrbit is true, rotate spring arm on Z axis; else reset to 0
  (set `RotatingMovementComponent.RotationRate` (`KismetMathLibrary.SelectRotator` (struct :`Yaw` 10.0) (struct) IsOrbiting) (`self.RotatingMovement`))
  (bind _output_get (set `SpringArmComponent.bInheritYaw` IsOrbiting (`self.SpringArm`)))
  (if (not _output_get)
    (`self.K2_SetActorRotation` (struct))))

(event `/Game/Blueprints/BattleObjects/BPI_DynamicCameraInterface.SetDynamicLocation`
  (params (Actor :type "Actor Object Reference") (Location :type "Vector Structure"))
  ; USING INTERFACE :: If the actor is a valid target, attach to it and look at it
  (`/Engine/EditorBlueprintResources/StandardMacros.IsValid` Actor
    (:`Is Valid`
      (`self.K2_AttachToActor` Actor "None" "SnapToTarget" "KeepRelative" "KeepRelative")
      (`SceneComponent.K2_SetRelativeRotation` :`self` (`self.Camera`)))
    (:`Is Not Valid`
      (set `self.TargetLocation` Location))))

(event `self.ReceiveTick`
  (params (DeltaSeconds :type "Float (single-precision)"))
  ; If not attached to anything, Viterp to location
  (`/Engine/EditorBlueprintResources/StandardMacros.IsValid` (`self.GetAttachParentActor`)
    (:`Is Not Valid`
      (`self.K2_SetActorLocation` (`KismetMathLibrary.VInterpTo` (`self.K2_GetActorLocation`) (`self.TargetLocation`) (`GameplayStatics.GetWorldDeltaSeconds`) 5.0)))))

(fn `UserConstructionScript`)